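; Base AI controller Blueprint for AI character variants.
; It starts the Brain component's logic on BeginPlay, then stops it and destroys the spatial and GA path components on UnPossess.
; Tick is empty, and disconnected leftover nodes hold unused experiments for pathing to the player or current target and choosing spatial positions.
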(event EventBeginPlay
  (|CallParentFunction)
  (AI|Logic|StartLogic (Variables|Default|GetBrainComponent)))

(event EventUnPossess
  (params (UnpossessedPawn :type Pawn%20Object%20Reference))
  (AI|Logic|StopLogic (Variables|Default|GetBrainComponent) "")
  (Components|DestroyComponent (Variables|Default|GetBP_SpatialComponent))
  (Components|DestroyComponent (Variables|Default|GetGAPathComponent)))

(event EventTick
  (params (DeltaSeconds :type Float%20%28single-precision%29)))

(fn ConstructionScript
  (|CallParentFunction))