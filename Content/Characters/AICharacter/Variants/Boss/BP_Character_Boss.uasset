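; Boss variant of the AI character that shows its own health bar on screen.
; On BeginPlay it runs the parent logic, creates a W_BossHealth widget, stores it and adds it to the viewport.
; It passes itself to the widget's UpdateHealthPercentage at start and again every Tick, so the bar refreshes by polling.
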(event EventBeginPlay
  (|CallParentFunction)
  (bind _returnvalue (UserInterface|CreateWidget "/Game/UI/W_BossHealth.W_BossHealth_C"))
  (bind _output_get (Variables|Default|SetBossHealthbarWidget _returnvalue))
  (UserInterface|Viewport|AddtoViewport _output_get 0)
  (Default|UpdateHealthPercentage _output_get self))

(event Collision|EventActorBeginOverlap
  (params (OtherActor :type Actor%20Object%20Reference))
  (|CallParentFunction OtherActor) ; This node is disabled and will not be called.\nDrag off pins to build functionality.
)

(event EventTick
  (params (DeltaSeconds :type Float%20%28single-precision%29))
  (|CallParentFunction DeltaSeconds)
  (Default|UpdateHealthPercentage (Variables|Default|GetBossHealthbarWidget) self))

(fn ConstructionScript
  (|CallParentFunction))